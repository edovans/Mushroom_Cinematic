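; BP_Dash_Volume_Fog is a mesh-based fog and cloud actor with adjustable look and wind motion.
; Its construction script creates dynamic instances of CloudMasterMaterial for seven cloud mesh components, two curved and five DashCloud.
; It pushes shared color, density, fading, brightness, contrast and wind variables into every instance.
; All work happens at construction, as the BeginPlay, overlap and Tick events are unused.
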(fn `UserConstructionScript`
  (bind _cloud_master_material (`self.Cloud_Master_Material`))
  (bind _returnvalue (`PrimitiveComponent.CreateDynamicMaterialInstance` (`self.Cloud_Curved_Mesh`) 0 _cloud_master_material "None"))
  (bind _returnvalue_2 (`PrimitiveComponent.CreateDynamicMaterialInstance` (`self.Dash_Cloud`) 0 _cloud_master_material "None"))
  (bind _returnvalue_3 (`PrimitiveComponent.CreateDynamicMaterialInstance` (`self.Cloud_Curved_Mesh1`) 0 _cloud_master_material "None"))
  (bind _returnvalue_4 (`PrimitiveComponent.CreateDynamicMaterialInstance` (`self.Dash_Cloud1`) 0 _cloud_master_material "None"))
  (bind _returnvalue_5 (`PrimitiveComponent.CreateDynamicMaterialInstance` (`self.Dash_Cloud2`) 0 _cloud_master_material "None"))
  (bind _returnvalue_6 (`PrimitiveComponent.CreateDynamicMaterialInstance` (`self.Dash_Cloud3`) 0 _cloud_master_material "None"))
  (bind _returnvalue_7 (`PrimitiveComponent.CreateDynamicMaterialInstance` (`self.Dash_Cloud4`) 0 _cloud_master_material "None"))
  (bind _output_get (set `self.NewVar_4` _returnvalue_7))
  (bind _output_get_2 (set `self.NewVar_3` _returnvalue_6))
  (bind _output_get_3 (set `self.NewVar_2` _returnvalue_5))
  (bind _output_get_4 (set `self.NewVar_1` _returnvalue_4))
  (bind _output_get_5 (set `self.NewVar_0` _returnvalue_3))
  (bind _output_get_6 (set `self.NewVar` _returnvalue_2))
  (bind _output_get_7 (set `self.Cloud_Material_Instance` _returnvalue))
  (`MaterialInstanceDynamic.SetVectorParameterValue` _output_get_7 "Base_Color_Tint" (`self.Cloud_Color`))
  (`MaterialInstanceDynamic.SetVectorParameterValue` _output_get_6 "Base_Color_Tint" (`self.Cloud_Color`))
  (`MaterialInstanceDynamic.SetVectorParameterValue` _output_get_5 "Base_Color_Tint" (`self.Cloud_Color`))
  (`MaterialInstanceDynamic.SetVectorParameterValue` _output_get_4 "Base_Color_Tint" (`self.Cloud_Color`))
  (`MaterialInstanceDynamic.SetVectorParameterValue` _output_get_3 "Base_Color_Tint" (`self.Cloud_Color`))
  (`MaterialInstanceDynamic.SetVectorParameterValue` _output_get_2 "Base_Color_Tint" (`self.Cloud_Color`))
  (`MaterialInstanceDynamic.SetVectorParameterValue` _output_get "Base_Color_Tint" (`self.Cloud_Color`))
  (`MaterialInstanceDynamic.SetScalarParameterValue` _output_get_7 "Distance_fade" (`self.Edge_Fading_Distance`))
  (`MaterialInstanceDynamic.SetScalarParameterValue` _output_get_6 "Distance_fade" (`self.Edge_Fading_Distance`))
  (`MaterialInstanceDynamic.SetScalarParameterValue` _output_get_5 "Distance_fade" (`self.Edge_Fading_Distance`))
  (`MaterialInstanceDynamic.SetScalarParameterValue` _output_get_4 "Distance_fade" (`self.Edge_Fading_Distance`))
  (`MaterialInstanceDynamic.SetScalarParameterValue` _output_get_3 "Distance_fade" (`self.Edge_Fading_Distance`))
  (`MaterialInstanceDynamic.SetScalarParameterValue` _output_get_2 "Distance_fade" (`self.Edge_Fading_Distance`))
  (`MaterialInstanceDynamic.SetScalarParameterValue` _output_get "Distance_fade" (`self.Edge_Fading_Distance`))
  (`MaterialInstanceDynamic.SetScalarParameterValue` _output_get_7 "Fog_Density" (`self.Cloud_Density`))
  (`MaterialInstanceDynamic.SetScalarParameterValue` _output_get_6 "Fog_Density" (`self.Cloud_Density`))
  (`MaterialInstanceDynamic.SetScalarParameterValue` _output_get_5 "Fog_Density" (`self.Cloud_Density`))
  (`MaterialInstanceDynamic.SetScalarParameterValue` _output_get_4 "Fog_Density" (`self.Cloud_Density`))
  (`MaterialInstanceDynamic.SetScalarParameterValue` _output_get_3 "Fog_Density" (`self.Cloud_Density`))
  (`MaterialInstanceDynamic.SetScalarParameterValue` _output_get_2 "Fog_Density" (`self.Cloud_Density`))
  (`MaterialInstanceDynamic.SetScalarParameterValue` _output_get "Fog_Density" (`self.Cloud_Density`))
  (`MaterialInstanceDynamic.SetScalarParameterValue` _output_get_7 "Camera_Fading_Distance" (`self.Camera_Fading_Distance`))
  (`MaterialInstanceDynamic.SetScalarParameterValue` _output_get_6 "Camera_Fading_Distance" (`self.Camera_Fading_Distance`))
  (`MaterialInstanceDynamic.SetScalarParameterValue` _output_get_5 "Camera_Fading_Distance" (`self.Camera_Fading_Distance`))
  (`MaterialInstanceDynamic.SetScalarParameterValue` _output_get_4 "Camera_Fading_Distance" (`self.Camera_Fading_Distance`))
  (`MaterialInstanceDynamic.SetScalarParameterValue` _output_get_3 "Camera_Fading_Distance" (`self.Camera_Fading_Distance`))
  (`MaterialInstanceDynamic.SetScalarParameterValue` _output_get_2 "Camera_Fading_Distance" (`self.Camera_Fading_Distance`))
  (`MaterialInstanceDynamic.SetScalarParameterValue` _output_get "Camera_Fading_Distance" (`self.Camera_Fading_Distance`))
  (`MaterialInstanceDynamic.SetScalarParameterValue` _output_get_7 "Emissive_Intensity" (`self.Cloud_Brightness`))
  (`MaterialInstanceDynamic.SetScalarParameterValue` _output_get_6 "Emissive_Intensity" (`self.Cloud_Brightness`))
  (`MaterialInstanceDynamic.SetScalarParameterValue` _output_get_5 "Emissive_Intensity" (`self.Cloud_Brightness`))
  (`MaterialInstanceDynamic.SetScalarParameterValue` _output_get_4 "Emissive_Intensity" (`self.Cloud_Brightness`))
  (`MaterialInstanceDynamic.SetScalarParameterValue` _output_get_3 "Emissive_Intensity" (`self.Cloud_Brightness`))
  (`MaterialInstanceDynamic.SetScalarParameterValue` _output_get_2 "Emissive_Intensity" (`self.Cloud_Brightness`))
  (`MaterialInstanceDynamic.SetScalarParameterValue` _output_get "Emissive_Intensity" (`self.Cloud_Brightness`))
  (`MaterialInstanceDynamic.SetScalarParameterValue` _output_get_7 "Wind_Velocity" (`self.Wind_Speed`))
  (`MaterialInstanceDynamic.SetScalarParameterValue` _output_get_6 "Wind_Velocity" (`self.Wind_Speed`))
  (`MaterialInstanceDynamic.SetScalarParameterValue` _output_get_5 "Wind_Velocity" (`self.Wind_Speed`))
  (`MaterialInstanceDynamic.SetScalarParameterValue` _output_get_4 "Wind_Velocity" (`self.Wind_Speed`))
  (`MaterialInstanceDynamic.SetScalarParameterValue` _output_get_3 "Wind_Velocity" (`self.Wind_Speed`))
  (`MaterialInstanceDynamic.SetScalarParameterValue` _output_get_2 "Wind_Velocity" (`self.Wind_Speed`))
  (`MaterialInstanceDynamic.SetScalarParameterValue` _output_get "Wind_Velocity" (`self.Wind_Speed`))
  (`MaterialInstanceDynamic.SetScalarParameterValue` _output_get_7 "Cloud_Wind_Tilling" (`self.Cloud_Wind_Tilling`))
  (`MaterialInstanceDynamic.SetScalarParameterValue` _output_get_6 "Cloud_Wind_Tilling" (`self.Cloud_Wind_Tilling`))
  (`MaterialInstanceDynamic.SetScalarParameterValue` _output_get_5 "Cloud_Wind_Tilling" (`self.Cloud_Wind_Tilling`))
  (`MaterialInstanceDynamic.SetScalarParameterValue` _output_get_4 "Cloud_Wind_Tilling" (`self.Cloud_Wind_Tilling`))
  (`MaterialInstanceDynamic.SetScalarParameterValue` _output_get_3 "Cloud_Wind_Tilling" (`self.Cloud_Wind_Tilling`))
  (`MaterialInstanceDynamic.SetScalarParameterValue` _output_get_2 "Cloud_Wind_Tilling" (`self.Cloud_Wind_Tilling`))
  (`MaterialInstanceDynamic.SetScalarParameterValue` _output_get "Cloud_Wind_Tilling" (`self.Cloud_Wind_Tilling`))
  (`MaterialInstanceDynamic.SetScalarParameterValue` _output_get_7 "Contrast_Intensity" (`self.Cloud_Contrast`))
  (`MaterialInstanceDynamic.SetScalarParameterValue` _output_get_6 "Contrast_Intensity" (`self.Cloud_Contrast`))
  (`MaterialInstanceDynamic.SetScalarParameterValue` _output_get_5 "Contrast_Intensity" (`self.Cloud_Contrast`))
  (`MaterialInstanceDynamic.SetScalarParameterValue` _output_get_4 "Contrast_Intensity" (`self.Cloud_Contrast`))
  (`MaterialInstanceDynamic.SetScalarParameterValue` _output_get_3 "Contrast_Intensity" (`self.Cloud_Contrast`))
  (`MaterialInstanceDynamic.SetScalarParameterValue` _output_get_2 "Contrast_Intensity" (`self.Cloud_Contrast`))
  (`MaterialInstanceDynamic.SetScalarParameterValue` _output_get "Contrast_Intensity" (`self.Cloud_Contrast`))
  (`MaterialInstanceDynamic.SetScalarParameterValue` _output_get "Wind_Direction" (`self.Wind_Direction`))
  (`MaterialInstanceDynamic.SetScalarParameterValue` _output_get_2 "Wind_Direction" (`self.Wind_Direction`))
  (`MaterialInstanceDynamic.SetScalarParameterValue` _output_get_3 "Wind_Direction" (`self.Wind_Direction`))
  (`MaterialInstanceDynamic.SetScalarParameterValue` _output_get_4 "Wind_Direction" (`self.Wind_Direction`))
  (`MaterialInstanceDynamic.SetScalarParameterValue` _output_get_5 "Wind_Direction" (`self.Wind_Direction`))
  (`MaterialInstanceDynamic.SetScalarParameterValue` _output_get_6 "Wind_Direction" (`self.Wind_Direction`))
  (`MaterialInstanceDynamic.SetScalarParameterValue` _output_get_7 "Wind_Direction" (`self.Wind_Direction`)))