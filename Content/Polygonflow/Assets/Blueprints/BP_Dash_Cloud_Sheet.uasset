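; BP_Dash_Cloud_Sheet is a placeable cloud sheet actor with adjustable look and wind.
; Its construction script creates a dynamic instance of the cloud master material on the DashCloud component's first slot.
; It then copies the actor's variables for tint, density, brightness, contrast, edge and camera fading, and wind into that material's parameters.
; The event graph has no active logic, so the Blueprint does nothing at runtime.
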(fn `UserConstructionScript`
  (bind _returnvalue (`PrimitiveComponent.CreateDynamicMaterialInstance` (`self.Dash_Cloud`) 0 (`self.Cloud_Master_Material`) "None"))
  (bind _output_get (set `self.Cloud_Material_Instance` _returnvalue))
  (`MaterialInstanceDynamic.SetVectorParameterValue` _output_get "Base_Color_Tint" (`self.Base Color Tint`))
  (`MaterialInstanceDynamic.SetScalarParameterValue` _output_get "Distance_fade" (`self.Edge Fading Distance`))
  (`MaterialInstanceDynamic.SetScalarParameterValue` _output_get "Fog_Density" (`self.Cloud_Density`))
  (`MaterialInstanceDynamic.SetScalarParameterValue` _output_get "Camera_Fading_Distance" (`self.Camera_Fading_Distance`))
  (`MaterialInstanceDynamic.SetScalarParameterValue` _output_get "Emissive_Intensity" (`self.Cloud Brightness`))
  (`MaterialInstanceDynamic.SetScalarParameterValue` _output_get "Wind_Velocity" (`self.Wind_Speed`))
  (`MaterialInstanceDynamic.SetScalarParameterValue` _output_get "Cloud_Wind_Tilling" (`self.Cloud_Wind_Tilling`))
  (`MaterialInstanceDynamic.SetScalarParameterValue` _output_get "Contrast_Intensity" (`self.Cloud_Contrast`))
  (`MaterialInstanceDynamic.SetScalarParameterValue` _output_get "Wind_Direction" (`self.Wind_Direction`)))